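; BP_DialogueTrigger is a one-shot trigger volume that starts a dialogue when the player character enters its collision component.
; On overlap it checks the DialogueActivation array in BP_RR_GameInstance at its DialogueIndex, so a line already played is skipped.
; Otherwise it marks that entry true, passes itself to the DialogueTinaGrace actor's DialoguePick, then destroys itself.
; Keeping the flags in the game instance lets played state outlast the actor and level loads.
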(event OnComponentBeginOverlap(CollisionComponent)
  (params (OverlappedComponent :type Primitive%20Component%20Object%20Reference) (OtherActor :type Actor%20Object%20Reference) (OtherComp :type Primitive%20Component%20Object%20Reference) (OtherBodyIndex :type Integer) (bFromSweep :type Boolean) (SweepResult :type Hit%20Result%20Structure%20%28by%20ref%29))
  (bind _dialogueindex (Variables|Default|GetDialogueIndex))
  (if (== OtherActor (Game|GetPlayerCharacter 0))
    (bind _asbp_rr_game_instance (Utilities|Casting|CastToBP_RR_GameInstance (Game|GetGameInstance)))
    (if (Utilities|Array|IsValidIndex (Variables|/Game/BP_RR_GameInstance.BP_RR_GameInstance_C|GetDialogueActivation _asbp_rr_game_instance) _dialogueindex)
      (if (not (Utilities|Array|Get(acopy) (Variables|/Game/BP_RR_GameInstance.BP_RR_GameInstance_C|GetDialogueActivation _asbp_rr_game_instance) _dialogueindex))
        (Utilities|Array|SetArrayElem (Variables|/Game/BP_RR_GameInstance.BP_RR_GameInstance_C|GetDialogueActivation _asbp_rr_game_instance) _dialogueindex true true)
        (bind _returnvalue (Actor|GetActorOfClass "/Game/Dialogue/DialogueTinaGrace.DialogueTinaGrace_C"))
        (Default|DialoguePick _returnvalue self)
        (Actor|DestroyActor)))))

(fn ConstructionScript)