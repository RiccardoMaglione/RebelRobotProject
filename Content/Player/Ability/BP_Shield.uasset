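; Player shield ability actor that blocks a limited number of projectiles and boosts the player's projectile speed with each block.
; Each overlapping projectile uses up a charge and extends Duration; non-final blocks destroy the projectile and compound a percentage speed bonus.
; Tick counts Duration down through a one-second Delay.
; Expiry or charge depletion restores the speed cached at BeginPlay and destroys the shield, but only expiry calls ShieldCooldown.
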(event OnComponentBeginOverlap(StaticMesh)
  (params (OverlappedComponent :type Primitive%20Component%20Object%20Reference) (OtherActor :type Actor%20Object%20Reference) (OtherComp :type Primitive%20Component%20Object%20Reference) (OtherBodyIndex :type Integer) (bFromSweep :type Boolean) (SweepResult :type Hit%20Result%20Structure%20%28by%20ref%29))
  (bind _asprojectile (Utilities|Casting|CastToProjectile (Components|GetOwner OtherComp)))
  (bind _output_get (Variables|Default|SetNumberOfBulletsCanBlock (- (Variables|Default|GetNumberOfBulletsCanBlock) 1.0)))
  (Variables|Default|SetDuration (+ (Variables|Default|GetDuration) 1.0))
  (Development|PrintString "Hello")
  (if (<= _output_get 0.0)
    (bind _asv4rrcharacter_1 (Utilities|Casting|CastToV4RRCharacter-1 (Game|GetPlayerCharacter 0)))
    (Utilities|Struct|SetmembersinWeaponStructure (Utilities|Array|Get(acopy) (Variables|/Game/Player/Weapon/ShootingComponent.ShootingComponent_C|GetWeaponStructureArray (Variables|/Game/V4RRCharacter-1.V4RRCharacter-1_C|GetShootingComponent _asv4rrcharacter_1)) (Variables|/Game/V4RRCharacter-1.V4RRCharacter-1_C|GetWeaponStructureIndex _asv4rrcharacter_1)) (Variables|Default|GetBasic_Projectile%20Speed))
    (Actor|DestroyActor)
    (else
      (bind _asv4rrcharacter_1_2 (Utilities|Casting|CastToV4RRCharacter-1 (Game|GetPlayerCharacter 0)))
      (Development|PrintString "Hello")
      (Utilities|Struct|SetmembersinWeaponStructure (Utilities|Array|Get(acopy) (Variables|/Game/Player/Weapon/ShootingComponent.ShootingComponent_C|GetWeaponStructureArray (Variables|/Game/V4RRCharacter-1.V4RRCharacter-1_C|GetShootingComponent _asv4rrcharacter_1_2)) (Variables|/Game/V4RRCharacter-1.V4RRCharacter-1_C|GetWeaponStructureIndex _asv4rrcharacter_1_2)) (+ (.ProjectileSpeed (Utilities|Struct|BreakWeaponStructure (Utilities|Array|Get(acopy) (Variables|/Game/Player/Weapon/ShootingComponent.ShootingComponent_C|GetWeaponStructureArray (Variables|/Game/V4RRCharacter-1.V4RRCharacter-1_C|GetShootingComponent _asv4rrcharacter_1_2)) (Variables|/Game/V4RRCharacter-1.V4RRCharacter-1_C|GetWeaponStructureIndex _asv4rrcharacter_1_2)))) (/ (* (.ProjectileSpeed (Utilities|Struct|BreakWeaponStructure (Utilities|Array|Get(acopy) (Variables|/Game/Player/Weapon/ShootingComponent.ShootingComponent_C|GetWeaponStructureArray (Variables|/Game/V4RRCharacter-1.V4RRCharacter-1_C|GetShootingComponent _asv4rrcharacter_1_2)) (Variables|/Game/V4RRCharacter-1.V4RRCharacter-1_C|GetWeaponStructureIndex _asv4rrcharacter_1_2)))) (Variables|Default|GetPercentualToAddAtSpeedBullets)) 1e+02)))
      (Development|PrintString (Utilities|String|ToString(Float) (+ (.ProjectileSpeed (Utilities|Struct|BreakWeaponStructure (Utilities|Array|Get(acopy) (Variables|/Game/Player/Weapon/ShootingComponent.ShootingComponent_C|GetWeaponStructureArray (Variables|/Game/V4RRCharacter-1.V4RRCharacter-1_C|GetShootingComponent _asv4rrcharacter_1_2)) (Variables|/Game/V4RRCharacter-1.V4RRCharacter-1_C|GetWeaponStructureIndex _asv4rrcharacter_1_2)))) (/ (* (.ProjectileSpeed (Utilities|Struct|BreakWeaponStructure (Utilities|Array|Get(acopy) (Variables|/Game/Player/Weapon/ShootingComponent.ShootingComponent_C|GetWeaponStructureArray (Variables|/Game/V4RRCharacter-1.V4RRCharacter-1_C|GetShootingComponent _asv4rrcharacter_1_2)) (Variables|/Game/V4RRCharacter-1.V4RRCharacter-1_C|GetWeaponStructureIndex _asv4rrcharacter_1_2)))) (Variables|Default|GetPercentualToAddAtSpeedBullets)) 1e+02))))
      (Actor|DestroyActor _asprojectile))))

(event EventBeginPlay
  (bind _asv4rrcharacter_1 (Utilities|Casting|CastToV4RRCharacter-1 (Game|GetPlayerCharacter 0)))
  (Variables|Default|SetBasic_Projectile%20Speed (.ProjectileSpeed (Utilities|Struct|BreakWeaponStructure (Utilities|Array|Get(acopy) (Variables|/Game/Player/Weapon/ShootingComponent.ShootingComponent_C|GetWeaponStructureArray (Variables|/Game/V4RRCharacter-1.V4RRCharacter-1_C|GetShootingComponent _asv4rrcharacter_1)) (Variables|/Game/V4RRCharacter-1.V4RRCharacter-1_C|GetWeaponStructureIndex _asv4rrcharacter_1))))))

(event EventTick
  (params (DeltaSeconds :type Float%20%28single-precision%29))
  (if (<= (Variables|Default|GetDuration) 0.0)
    (bind _asv4rrcharacter_1 (Utilities|Casting|CastToV4RRCharacter-1 (Game|GetPlayerCharacter 0)))
    (Utilities|Struct|SetmembersinWeaponStructure (Utilities|Array|Get(acopy) (Variables|/Game/Player/Weapon/ShootingComponent.ShootingComponent_C|GetWeaponStructureArray (Variables|/Game/V4RRCharacter-1.V4RRCharacter-1_C|GetShootingComponent _asv4rrcharacter_1)) (Variables|/Game/V4RRCharacter-1.V4RRCharacter-1_C|GetWeaponStructureIndex _asv4rrcharacter_1)) (Variables|Default|GetBasic_Projectile%20Speed))
    (Default|ShieldCooldown _asv4rrcharacter_1 (Variables|/Game/Player/Ability/AbilityComponent.AbilityComponent_C|GetAC_Cooldown_Shield (Variables|/Game/V4RRCharacter-1.V4RRCharacter-1_C|GetAbilityComponent _asv4rrcharacter_1)))
    (Actor|DestroyActor)
    (else
      (Utilities|FlowControl|Delay 1.0)
      (bind _output_get (Variables|Default|SetDuration (- (Variables|Default|GetDuration) 1.0)))
      (Development|PrintString (Utilities|String|ToString(Float) _output_get)))))

(fn ConstructionScript)