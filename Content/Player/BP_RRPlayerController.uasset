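; Player controller that restores saved audio volume and provides a level restart key.
; On BeginPlay it loads the VolumeGeneral SaveVolume slot, if present, and applies its general volume to the TOT bus.
; Pressing P reopens the current level, passing PSAStore from BP_RR_GameInstance as the travel options.
; Similar music (AMB bus) and SFX (also TOT bus) restore chains exist but are disconnected, so never run.
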(event EventBeginPlay
  (bind _returnvalue (SaveGame|DoesSaveGameExist "VolumeGeneral"))
  (if _returnvalue
    (bind _returnvalue_2 (SaveGame|LoadGamefromSlot "VolumeGeneral"))
    (bind _assave_volume (Utilities|Casting|CastToSaveVolume _returnvalue_2))
    (Class|FMODBlueprintStatics|BusSetVolume "/Game/FMOD/Buses/TOT.TOT" (Variables|/Game/NewUI/SaveVolume.SaveVolume_C|GetGeneralVolumeSave _assave_volume))))

(event EventTick
  (params (DeltaSeconds :type Float%20%28single-precision%29)))

(event Input|KeyboardEvents|P
  (params (Key :type Key%20Structure :default "None"))
  (:Pressed
    (bind _returnvalue (Game|GetCurrentLevelName true))
    (bind _asbp_rr_game_instance (Utilities|Casting|CastToBP_RR_GameInstance (Game|GetGameInstance)))
    (Game|OpenLevel(byName) (Utilities|String|StringToName _returnvalue) true (Variables|/Game/BP_RR_GameInstance.BP_RR_GameInstance_C|GetPSAStore _asbp_rr_game_instance))))

(fn ConstructionScript)