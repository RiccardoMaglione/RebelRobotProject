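; Explosive barrel that detonates when hit by a player projectile or kamikaze explosion, or when a nearby barrel's blast triggers it.
; Two sequential timelines grow area indicators as a warning before the blast.
; The explosion damages enemies, damages and flags the player dead, and chains other barrels in range through a flag polled on Tick.
; It shakes the player's camera, spawns particles and a random-sized decal, then destroys itself.
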(event OnComponentBeginOverlap(Box)
  (params (OverlappedComponent :type Primitive%20Component%20Object%20Reference) (OtherActor :type Actor%20Object%20Reference) (OtherComp :type Primitive%20Component%20Object%20Reference) (OtherBodyIndex :type Integer) (bFromSweep :type Boolean) (SweepResult :type Hit%20Result%20Structure%20%28by%20ref%29))
  (Utilities|FlowControl|Sequence
    (:then_0
      (if (Actor|ActorHasTag OtherActor (Variables|Default|GetPlayerProjectileTag))
        (if (not (Variables|Default|GetisExploding)) :!label _label
          (Variables|Default|SetisExploding true)
          (Utilities|FlowControl|DoOnce false
            (:Completed
              (CallFunction|FirstFeed))))))
    (:then_1
      (if (Actor|ActorHasTag OtherActor (Variables|Default|GetKamikazeExplosionTag))
        (goto _label)))))

(event Custom|FirstFeed
  (bind _alpha (Timeline|FirstFeedTimeline PlayFromStart)
    (:Update
      (Transformation|SetRelativeScale3D (Variables|Default|GetExplosiveAreaFeed) (Math|Vector|Lerp(Vector) "0, 0, 0" "0.340000,0.340000,0.340000" _alpha)))
    (:Finished
      (CallFunction|SecondFeed))))

(event Custom|SecondFeed
  (bind _alpha (Timeline|SecondFeedTimeline PlayFromStart)
    (:Update
      (Transformation|SetRelativeScale3D (Variables|Default|GetExplosiveAreaExpandFeed) (Math|Vector|Lerp(Vector) "0, 0, 0" "0.340000,0.340000,0.340000" _alpha)))
    (:Finished
      (CallFunction|Explode))))

(event EventTick
  (params (DeltaSeconds :type Float%20%28single-precision%29))
  (|CallParentFunction DeltaSeconds)
  (if (Variables|Default|GetexplodeOrder)
    (if (not (Variables|Default|GetisExploding))
      (Variables|Default|SetisExploding true)
      (Utilities|FlowControl|DoOnce false
        (:Completed
          (CallFunction|FirstFeed))))))

(fn ConstructionScript
  (|CallParentFunction))

(fn Explode
  (bind _returnvalue (Transformation|GetActorLocation))
  (bind _area (Variables|Default|GetArea))
  (for _array_element (Collision|GetOverlappingActors _area "/Game/V4RRCharacter-1.V4RRCharacter-1_C" :!class /Script/Engine.PrimitiveComponent)
    (bind _asv4rrcharacter_1 (Utilities|Casting|CastToV4RRCharacter-1 _array_element))
    (Variables|/Game/V4RRCharacter-1.V4RRCharacter-1_C|SetPlayer_Health _asv4rrcharacter_1 (- (Variables|/Game/V4RRCharacter-1.V4RRCharacter-1_C|GetPlayer_Health _asv4rrcharacter_1) (Variables|Default|GetdamageToPlayer)))
    (Variables|/Game/V4RRCharacter-1.V4RRCharacter-1_C|SetIsDeath _asv4rrcharacter_1 true))
  (for _array_element_2 (Collision|GetOverlappingActors _area "/Game/AI/AI_Base_Folder/AIRRCharacter.AIRRCharacter_C" :!class /Script/Engine.PrimitiveComponent)
    (bind _asairrcharacter (Utilities|Casting|CastToAIRRCharacter _array_element_2))
    (bind _output_get (Variables|/Game/AI/AI_Base_Folder/AIRRCharacter.AIRRCharacter_C|SetAI_Base_Life _asairrcharacter (- (Variables|/Game/AI/AI_Base_Folder/AIRRCharacter.AIRRCharacter_C|GetAI_Base_Life _asairrcharacter) (Variables|Default|GetdamageToEnemy))))
    (if (<= _output_get 0.0)
      (Default|Death? _asairrcharacter)))
  (for _array_element_3 (Collision|GetOverlappingActors _area "BP_ExplosiveBarrel_C" :!class /Script/Engine.PrimitiveComponent)
    (bind _asbp_explosive_barrel (Utilities|Casting|CastToBP_ExplosiveBarrel _array_element_3))
    (Variables|BP_ExplosiveBarrel_C|SetexplodeOrder _asbp_explosive_barrel true))
  (bind _asv4rrcharacter_1_2 (Utilities|Casting|CastToV4RRCharacter-1 (Game|GetPlayerCharacter 0)))
  (Camera|PlayWorldCameraShake "/Game/Camera/ExplosionShakeBlueprint.ExplosionShakeBlueprint_C" (Transformation|GetWorldLocation (Variables|/Game/V4RRCharacter-1.V4RRCharacter-1_C|GetRR_CameraComponent _asv4rrcharacter_1_2)) 1e+02 1e+02)
  (Effects|SpawnEmitteratLocation "/Game/LPSPSample/Art/Effects/PS_Explosion.PS_Explosion" _returnvalue (Transformation|GetActorRotation) "2.000000,2.000000,2.000000")
  (Rendering|Decal|SpawnDecalatLocation "/Game/LPSPSample/Art/Effects/MI_Decal_Explosion_001.MI_Decal_Explosion_001" (Math|Conversions|ToVector(Float) (Math|Random|RandomFloatinRange 4e+02 5e+02)) _returnvalue "-90.000000,0.000000,0.000000" 0.0)
  (Actor|DestroyActor))